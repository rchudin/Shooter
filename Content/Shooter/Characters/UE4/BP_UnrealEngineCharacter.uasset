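; Shooter character Blueprint that arms itself with an M16 shortly after spawning, with all BeginPlay logic running only on the authority.
; Outside standalone games, the authority destroys the character's Mesh component.
; After a short delay, it spawns BP_M16 at the first-person camera's location and passes it to the WeaponManager through TakeWeapon.
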(event `self.ReceiveBeginPlay`
  (`|ExecutionSequence`
    (:`then_0`
      (`/Engine/EditorBlueprintResources/ActorMacros.Switch Has Authority`
        (:`Authority`
          (if (not (`KismetSystemLibrary.IsStandalone`))
            (`ActorComponent.K2_DestroyComponent` (`self.Mesh`))))))
    (:`then_1`
      (`/Engine/EditorBlueprintResources/ActorMacros.Switch Has Authority`
        (:`Authority`
          (`KismetSystemLibrary.Delay` 3.0)
          (bind _returnvalue (`|SpawnActorFromClass` "/Game/Shooter/Weapon/M16/BP_M16.BP_M16_C" (`KismetMathLibrary.MakeTransform` (`SceneComponent.GetSocketLocation` (`self.FirstPersonCamera`) "None")) "AlwaysSpawn" "OverrideRootScale" null null))
          (`WeaponManager.TakeWeapon` (`self.WeaponManager`) _returnvalue))))))

(fn `UserConstructionScript`)